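; BP_Spawner is a spawner actor that places a single Bp_EnemyBase enemy at its own location and rotation.
; On BeginPlay, AttemptToSpawn checks whether CurrentEnemy is valid and only prints a debug message if one already exists.
; Otherwise SpawnEnemy spawns the enemy, adjusting for collisions but always spawning, and stores it in CurrentEnemy.
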(event EventBeginPlay
  (CallFunction|AttempttoSpawn))

(fn ConstructionScript)

(fn AttempttoSpawn
  (Utilities|IsValid (Variables|Default|GetCurrentEnemy)
    (:Is%20Valid
      (Development|PrintString "Enemy Already Sapwned"))
    (:Is%20Not%20Valid
      (CallFunction|SpawnEnemy))))

(fn SpawnEnemy
  (bind _returnvalue (Game|SpawnActorfromClass "/Game/New_Assets/Blueprints/Bp_EnemyBase.Bp_EnemyBase_C" (Math|Transform|MakeTransform (Transformation|GetActorLocation) (Transformation|GetActorRotation)) "AdjustIfPossibleButAlwaysSpawn" 0 0))
  (Variables|Default|SetCurrentEnemy _returnvalue))