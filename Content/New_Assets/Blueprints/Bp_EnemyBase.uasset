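; Base enemy actor that moves steadily along the negative world X axis, getting faster as the game's skill level rises.
; On BeginPlay it finds and caches the GameManager actors in the level.
; Each Tick it does a swept location update, scaling delta time by its own speed value plus the first GameManager's SkillLevel.
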(event EventTick
  (params (DeltaSeconds :type Float%20%28single-precision%29))
  (bind _returnvalue (Transformation|GetActorLocation))
  (Transformation|SetActorLocation (Math|Vector|MakeVector (- (.x _returnvalue) (* DeltaSeconds (+ (Variables|Default|GetSpeed%20Multiplye) (Variables|/Game/TwinStickBP/Blueprints/GameManager.GameManager_C|GetSkill%20level (Utilities|Array|Get(acopy) (stale EventBeginPlay _outactors)))))) (.y _returnvalue) (.z _returnvalue)) true false))

(event EventBeginPlay
  (bind _outactors (Actor|GetAllActorsOfClass "/Game/TwinStickBP/Blueprints/GameManager.GameManager_C")))

(fn ConstructionScript)